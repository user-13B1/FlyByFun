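; Player controller for the airplane pawn that sets up input and owns the flight HUD.
; On BeginPlay it adds the default Enhanced Input mapping context, creates the VehicleUI widget in non-MPH mode, and caches the controlled AirPlanePawn.
; UpdateHeals forwards a value to the HUD.
; A HUD speed update from the pawn exists but is disconnected, and Tick is empty.
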(event EventBeginPlay
  (Input|AddMappingContext (PlayerController|LocalPlayerSubsystems|GetEnhancedInputLocalPlayerSubsystem) "/Game/AirPlane/IMC_Default.IMC_Default" 0 "(bIgnoreAllPressedKeysUntilRelease=True,bForceImmediately=False)") ; Adding the Input Mapping Context needed to trigger the proper Input Actions.
  (bind _returnvalue (UserInterface|CreateWidget "/Game/UI/VehicleUI.VehicleUI_C" self))
  (bind _output_get (Variables|Default|SetAirPlaneHUD _returnvalue))
  (UserInterface|Viewport|AddtoViewport _output_get 0)
  (bind _asair_plane_pawn (Utilities|Casting|CastToAirPlanePawn (Pawn|GetControlledPawn)))
  (Variables|Default|SetAirPlanePawn _asair_plane_pawn))

(event EventTick
  (params (DeltaSeconds :type Float%20%28single-precision%29)))

(fn ConstructionScript)

(fn UpdateHeals
  (params (Value :type Integer))
  (Default|UpdateHeals (Variables|Default|GetAirPlaneHUD) Value))