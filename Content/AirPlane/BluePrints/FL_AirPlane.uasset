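; Airplane function library with a helper that adds random bullet dispersion to a rotator.
; AddBulletDispersion offsets pitch and yaw by random amounts within plus or minus the given value and leaves roll unchanged.
; The pitch offset is also scaled by the cosine of another normalized random value, pulling vertical spread slightly toward the center.
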(fn AddBulletDispersion
  (params (Value :type Float%20%28double-precision%29) (InputRoll :type Rotator))
  (bind (_roll _pitch _yaw) (Math|Rotator|BreakRotator InputRoll))
  (bind _returnvalue (- 0.0 Value))
  (bind _returnvalue_2 (Math|Random|RandomFloatinRange _returnvalue Value))
  (return (Math|Rotator|MakeRotator _roll (+ _pitch (* (Math|Random|RandomFloatinRange Value _returnvalue) (Math|Trig|Cos(Radians) (/ _returnvalue_2 Value)))) (+ _yaw _returnvalue_2))))