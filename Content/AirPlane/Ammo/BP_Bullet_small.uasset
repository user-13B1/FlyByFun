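; Small airplane bullet actor that destroys itself one second after spawning.
; On hit, it sends HitMessage with its Power to the struck actor and applies a fixed upward impulse to physics-simulating components.
; It spawns a scaled-down bomb explosion at the hit location and sends DestroyItMessage to actors implementing I_AirPlane.
; The impact sound node is disconnected and never plays.
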(event EventBeginPlay
  (bind _self self)
  (Utilities|FlowControl|Delay 1.0)
  (Utilities|IsValid _self
    (:Is%20Valid
      (Actor|DestroyActor _self))))

(event Collision|EventActorBeginOverlap
  (params (OtherActor :type Actor%20Object%20Reference)))

(event EventTick
  (params (DeltaSeconds :type Float%20%28single-precision%29)))

(event Collision|EventHit
  (params (MyComp :type Primitive%20Component%20Object%20Reference) (Other :type Actor%20Object%20Reference) (OtherComp :type Primitive%20Component%20Object%20Reference) (bSelfMoved :type Boolean) (HitLocation :type Vector :default "0, 0, 0") (HitNormal :type Vector :default "0, 0, 0") (NormalImpulse :type Vector :default "0, 0, 0") (Hit :type Hit%20Result%20Structure%20%28by%20ref%29))
  (Variables|Default|Sethit_location HitLocation)
  (Utilities|FlowControl|Sequence
    (:then_0
      (Class|IAirPlane|Hit(Message) Other 0.0 (Variables|Default|GetPower)))
    (:then_1
      (if (Physics|IsSimulatingPhysics OtherComp "None")
        (Physics|AddImpulseatLocation OtherComp "0.000000,0.000000,1333.000000" "0, 0, 0" "None")))
    (:then_2
      (Effects|SpawnEmitteratLocation "/Game/ExampleContent/Blueprint_Communication/Effects/P_Explosion_Bomb.P_Explosion_Bomb" HitLocation "0, 0, 0" "0.200000,0.200000,0.200000")
      (if (Utilities|DoesObjectImplementInterface Other "/Game/BluePrint/I_AirPlane.I_AirPlane_C")
        (Class|IAirPlane|DestroyIt(Message) Other)))))

(fn ConstructionScript)