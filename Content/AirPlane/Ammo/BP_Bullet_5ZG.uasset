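; BP_Bullet_5ZG is an airplane bullet projectile that destroys itself one second after spawning or shortly after bouncing.
; On hit, it pushes physics-simulating components upward with an impulse, otherwise sends the other actor a hit message carrying slightly randomized Power.
; Every hit spawns a bomb explosion effect.
; Actors implementing I_AirPlane also receive a destroy message, and the bullet is removed immediately.
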(event OnProjectileBounce(ProjectileMovement)
  (params (ImpactResult :type Hit%20Result%20Structure%20%28by%20ref%29) (ImpactVelocity :type Vector%20%28by%20ref%29 :default "0, 0, 0"))
  (Utilities|FlowControl|Delay 0.1)
  (Actor|DestroyActor self))

(event EventBeginPlay
  (bind _self self)
  (Utilities|FlowControl|Delay 1.0)
  (Utilities|IsValid _self
    (:Is%20Valid
      (Actor|DestroyActor _self))))

(event Collision|EventActorBeginOverlap
  (params (OtherActor :type Actor%20Object%20Reference)))

(event EventTick
  (params (DeltaSeconds :type Float%20%28single-precision%29)))

(event Collision|EventHit
  (params (MyComp :type Primitive%20Component%20Object%20Reference) (Other :type Actor%20Object%20Reference) (OtherComp :type Primitive%20Component%20Object%20Reference) (bSelfMoved :type Boolean) (HitLocation :type Vector :default "0, 0, 0") (HitNormal :type Vector :default "0, 0, 0") (NormalImpulse :type Vector :default "0, 0, 0") (Hit :type Hit%20Result%20Structure%20%28by%20ref%29))
  (Variables|Default|Sethit_location HitLocation)
  (if (Physics|IsSimulatingPhysics OtherComp "None")
    (Physics|AddImpulseatLocation OtherComp "0.000000,0.000000,1333.000000" "0, 0, 0" "None")
    (else
      (Class|IAirPlane|Hit(Message) Other (Math|Conversions|ToFloat(Integer) (+ (Variables|Default|GetPower) (Math|Random|RandomIntegerinRange -1 1))))))
  (Effects|SpawnEmitteratLocation "/Game/ExampleContent/Blueprint_Communication/Effects/P_Explosion_Bomb.P_Explosion_Bomb" (Variables|Default|Gethit_location) "0, 0, 0" "0.500000,0.500000,3.000000")
  (if (Utilities|DoesObjectImplementInterface Other "/Game/AirPlane/I_AirPlane.I_AirPlane_C")
    (Class|IAirPlane|DestroyIt(Message) Other)
    (Actor|DestroyActor self)))

(fn ConstructionScript)