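; Airplane bomb actor that moves by projectile movement, with its initial speed set in the construction script.
; On hit it spawns an explosion effect at the impact point.
; If its mesh still exists, it destroys that component and sends DestroyItMessage to actors overlapping RadiusDamge that implement I_AirPlane.
; The mesh validity check limits the blast to one time, though the actor itself is never destroyed here.
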(event EventBeginPlay)

(event Collision|EventActorBeginOverlap
  (params (OtherActor :type Actor%20Object%20Reference)))

(event EventTick
  (params (DeltaSeconds :type Float%20%28single-precision%29)))

(event Collision|EventHit
  (params (MyComp :type Primitive%20Component%20Object%20Reference) (Other :type Actor%20Object%20Reference) (OtherComp :type Primitive%20Component%20Object%20Reference) (bSelfMoved :type Boolean) (HitLocation :type Vector :default "0, 0, 0") (HitNormal :type Vector :default "0, 0, 0") (NormalImpulse :type Vector :default "0, 0, 0") (Hit :type Hit%20Result%20Structure%20%28by%20ref%29))
  (bind _sm_prototype_bomb_a (Variables|Default|GetSM_Prototype_Bomb_A))
  (Effects|SpawnEmitteratLocation "/Game/ExampleContent/Blueprint_Communication/Effects/P_Explosion_Bomb.P_Explosion_Bomb" HitLocation)
  (Utilities|IsValid _sm_prototype_bomb_a
    (:Is%20Valid
      (Components|DestroyComponent _sm_prototype_bomb_a)
      (for _array_element (Collision|GetOverlappingActors (Variables|Default|GetRadiusDamge) 0 :!class /Script/Engine.PrimitiveComponent)
        (if (Utilities|DoesObjectImplementInterface _array_element "/Game/AirPlane/I_AirPlane.I_AirPlane_C")
          (Class|IAirPlane|DestroyIt(Message) _array_element))))))

(fn ConstructionScript
  (CallFunction|SetSpeed (Variables|Default|GetInitial%20Speed)))

(fn SetSpeed
  (params (Initial%20Speed :type Float%20%28single-precision%29))
  (Variables|/Script/Engine.ProjectileMovementComponent|SetInitialSpeed (Variables|Default|GetProjectileMovement) Initial%20Speed))