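; Airplane machine gun actor that fires BP_Bullet_5ZG projectiles while shooting is switched on.
; SetShoot toggles actor tick, and a Delay inside Tick throttles the shot rate.
; Each shot rotates the GunClip component a step and spawns a bullet at the Arrow component, with random-spread aim from AddBulletDispersion applied to the Arrow's rotation.
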(event EventBeginPlay)

(event Collision|EventActorBeginOverlap
  (params (OtherActor :type Actor%20Object%20Reference)))

(event EventTick
  (params (DeltaSeconds :type Float%20%28single-precision%29))
  (bind _arrow (Variables|Default|GetArrow))
  (Utilities|FlowControl|Delay 0.3)
  (Transformation|AddRelativeRotation (Variables|Default|GetGunClip) "0.000000,0.000000,6.000000" false false)
  (bind _outpurroll (CallFunction|AddBulletDispersion 0.6 (Transformation|GetWorldRotation _arrow)))
  (Game|SpawnActorfromClass "/Game/AirPlane/Ammo/BP_Bullet_5ZG.BP_Bullet_5ZG_C" (Math|Transform|MakeTransform (Transformation|GetWorldLocation _arrow) _outpurroll) "Undefined" 0 0))

(event EventSetShoot
  (params (Value :type Boolean))
  (Actor|Tick|SetActorTickEnabled Value))

(fn ConstructionScript)