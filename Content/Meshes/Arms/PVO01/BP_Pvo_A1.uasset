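; BP_Pvo_A1 is an anti-air (PVO) gun turret that turns to track the player's pawn.
; Each Tick sets the gun head's world yaw from a look-at rotation toward the player.
; Barrel pitching and randomly delayed firing of BP_Bullet_Medium with dispersion from the Arrow component exist in the graph but are disconnected, so it never shoots.
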(event EventBeginPlay)

(event Collision|EventActorBeginOverlap
  (params (OtherActor :type Actor%20Object%20Reference)))

(event EventTick
  (params (DeltaSeconds :type Float%20%28single-precision%29))
  (Transformation|SetWorldRotation (Variables|Default|GetSM_PvoGun_Head) (Math|Rotator|MakeRotator 0.0 0.0 (.Yaw (Math|Rotator|BreakRotator (Math|Rotator|FindLookatRotation (Transformation|GetWorldLocation (Variables|Default|GetSM_PvoGun_Head)) (Transformation|GetActorLocation (Game|Player|GetPlayerPawn 0)))))) false false))

(fn ConstructionScript)