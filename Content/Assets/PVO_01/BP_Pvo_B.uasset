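; BP_Pvo_B is an air-defense gun turret that continuously tracks the player pawn and fires at it.
; Each Tick yaws the gun head and pitches the trunk toward the player using separate look-at rotations.
; A randomized Delay on Tick throttles fire to roughly twice a second, spawning BP_Bullet_Medium at the Arrow with added dispersion.
; It has no range or line-of-sight check.
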(event EventBeginPlay)

(event Collision|EventActorBeginOverlap
  (params (OtherActor :type Actor%20Object%20Reference)))

(event EventTick
  (params (DeltaSeconds :type Float%20%28single-precision%29))
  (bind _arrow (Variables|Default|GetArrow))
  (Transformation|SetWorldRotation (Variables|Default|GetSM_PvoGun_Head) (Math|Rotator|MakeRotator 0.0 0.0 (.Yaw (Math|Rotator|BreakRotator (Math|Rotator|FindLookatRotation (Transformation|GetWorldLocation (Variables|Default|GetSM_PvoGun_Head)) (Transformation|GetActorLocation (Game|Player|GetPlayerPawn 0)))))) false false)
  (Transformation|SetRelativeRotation (Variables|Default|GetSM_PvoGun_Trunk) (Math|Rotator|MakeRotator 0.0 (.Pitch (Math|Rotator|BreakRotator (Math|Rotator|FindLookatRotation (Transformation|GetWorldLocation (Variables|Default|GetSM_PvoGun_Trunk)) (Transformation|GetActorLocation (Game|Player|GetPlayerPawn 0))))) 0.0) false false)
  (Utilities|FlowControl|Delay (+ 0.5 (Math|Random|RandomFloatinRange 0.0 0.2)))
  (bind _outpurroll (CallFunction|AddBulletDispersion 0.3 (Transformation|GetWorldRotation _arrow)))
  (Game|SpawnActorfromClass "/Game/AirPlane/Ammo/BP_Bullet_Medium.BP_Bullet_Medium_C" (Math|Transform|MakeTransform (Transformation|GetWorldLocation _arrow) _outpurroll) "AdjustIfPossibleButDontSpawnIfColliding" 0 0))

(fn ConstructionScript)