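; BP_SplashStartScreen is a 3, 2, 1, Go countdown splash, triggered by the StartNewGame event.
; StartNewGame unhides the 3 mesh, then passes each number mesh in turn to a shared Start event, waiting TimePlayOne before each.
; Start makes the mesh visible, scales it by the TimelineSplash Action curve times Size, and hides it when the timeline finishes.
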(event Custom|Start
  (params (Mesh :type Static%20Mesh%20Component%20Object%20Reference))
  (Rendering|SetVisibility Mesh true false)
  (bind _action (Timeline|TimelineSplash PlayFromStart)
    (:Update
      (Transformation|SetRelativeScale3D Mesh (* _action (Variables|Default|GetSize))))
    (:Finished
      (Rendering|SetVisibility Mesh false false))))

(event EventStartNewGame
  (Development|SetHiddeninGame (Variables|Default|GetSM_Number_3) false false)
  (Utilities|FlowControl|Delay (Variables|Default|GetTimePlayOne))
  (CallFunction|Start (Variables|Default|GetSM_Number_3))
  (Utilities|FlowControl|Delay (Variables|Default|GetTimePlayOne))
  (CallFunction|Start (Variables|Default|GetSM_Number_2))
  (Utilities|FlowControl|Delay (Variables|Default|GetTimePlayOne))
  (CallFunction|Start (Variables|Default|GetSM_Number_1))
  (Utilities|FlowControl|Delay (Variables|Default|GetTimePlayOne))
  (CallFunction|Start (Variables|Default|GetSM_Number_Go)))

(fn ConstructionScript)