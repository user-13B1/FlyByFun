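; Anti-aircraft turret that tracks the player's plane and takes damage through a health widget until it is destroyed.
; Tick checks Eyesight range, interpolates head yaw and trunk pitch toward the plane, then calls Fire through a Delay.
; SpawnBullet only computes a dispersed rotation without spawning a projectile.
; Death removes the turret's components, while recoil animation and demolition effects are present but never run.
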(event Custom|Fire
  ;[1 1 1] Comment
  (CallFunction|SpawnBullet))

(event EventBeginPlay
  ;[1 1 1] Comment
  (bind _ascasual_air_plain_pawn (Utilities|Casting|CastToCasualAirPlainPawn (Game|Player|GetPlayerPawn 0)))
  (Variables|Default|SetAirPlainPawn _ascasual_air_plain_pawn)
  (bind _asw_pvo_heals (Utilities|Casting|CastToW_PVO_Heals (UserInterface|GetWidget (Variables|Default|GetWidget))))
  (Variables|Default|SetWidgetHeals _asw_pvo_heals))

(event Collision|EventActorBeginOverlap
  (params (OtherActor :type Actor%20Object%20Reference)))

(event EventTick
  (params (DeltaSeconds :type Float%20%28single-precision%29))
  (if (and (Variables|Default|GetIsGame) (Variables|Default|GetIsLive))
    (bind _newparam (CallFunction|IsEyeSight))
    (if _newparam
      (CallFunction|UpdateHeadRotation DeltaSeconds)
      (CallFunction|UpdateArmsRotation DeltaSeconds)
      (Utilities|FlowControl|Delay (Variables|Default|GetDelayFire))
      (CallFunction|Fire)
      (Variables|Default|SetDelayFire (Variables|Default|GetRateFire)))))

(event EventStopGame
  ;[1 1 1] Comment
  (Actor|Tick|SetActorTickEnabled false)
  (Variables|Default|SetIsGame false))

(event EventHit
  (params (Power :type Integer))
  (if (and (Variables|Default|GetIsGame) (Variables|Default|GetIsLive))
    (bind _output_get (Variables|Default|SetHeals (- (Variables|Default|GetHeals) Power)))
    (Default|SetHealsValue (Variables|Default|GetWidgetHeals) _output_get)
    (if (<= (Variables|Default|GetHeals) 0)
      (CallFunction|Death))))

(event EventStartNewGame
  ;[1 1 1] Comment
  (Actor|Tick|SetActorTickEnabled true))

(fn ConstructionScript
  (bind _trunk (Variables|Default|GetTrunk))
  (bind _relativelocation (Variables|/Script/Engine.SceneComponent|GetRelativeLocation _trunk))
  (bind (_x _y _z) (Math|Vector|BreakVector _relativelocation))
  (Variables|Default|SetTrunkStartLocation _relativelocation)
  (Variables|Default|SetTrunkRecoilOffsetLocation (Math|Vector|MakeVector (+ _x -4e+01) _y _z)))

(fn IsEyeSight
  (return (> (Variables|Default|GetEyesight) (Math|Vector|Distance(Vector) (Transformation|GetWorldLocation (Variables|Default|GetDefaultSceneRoot)) (Default|GetAirPlaneWorldLocation (Variables|Default|GetAirPlainPawn))))))

(fn UpdateHeadRotation
  (params (Delata :type Float%20%28double-precision%29))
  (Transformation|SetWorldRotation (Variables|Default|GetHead) (Math|Rotator|MakeRotator 0.0 0.0 (.yaw (Math|Interpolation|RInterpTo (Transformation|GetWorldRotation (Variables|Default|GetHead)) (Math|Rotator|FindLookatRotation (Transformation|GetWorldLocation (Variables|Default|GetHead)) (Default|GetAirPlaneWorldLocation (Variables|Default|GetAirPlainPawn))) Delata 1.5))) false false))

(fn UpdateArmsRotation
  (params (Delta :type Float%20%28double-precision%29))
  (bind _trunk (Variables|Default|GetTrunk))
  (Transformation|SetRelativeRotation (Variables|Default|GetTrunk) (Math|Rotator|MakeRotator 0.0 (.pitch (Math|Interpolation|RInterpTo (Transformation|GetWorldRotation _trunk) (Math|Rotator|FindLookatRotation (Transformation|GetWorldLocation _trunk) (Default|GetAirPlaneWorldLocation (Variables|Default|GetAirPlainPawn))) Delta 2.0)) 0.0) false false))

(fn SpawnBullet
  (if (Math|Boolean|ANDBoolean (Variables|Default|GetIsGame) (Variables|Default|GetIsLive) (Utilities|IsValid (Variables|Default|GetArrow)))
    (bind _outpurroll (CallFunction|AddBulletDispersion 0.3 (Transformation|GetWorldRotation (Variables|Default|GetArrow))))))

(fn Death
  (Actor|Tick|SetActorTickEnabled false)
  (Variables|Default|SetIsLive false)
  (Components|DestroyComponent (Variables|Default|GetWidget))
  (Components|DestroyComponent (Variables|Default|GetTrunk))
  (Components|DestroyComponent (Variables|Default|GetHead)))