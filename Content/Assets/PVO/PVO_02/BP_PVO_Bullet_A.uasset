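; BP_PVO_Bullet_A is an anti-air bullet actor that damages airplanes and destroys itself 0.8 seconds after spawning.
; On hit it plays an impact sound and explosion effect, then sends slightly randomized PowerHit damage through the I_AirPlane interface's HitMessage.
; Physics-simulated components also receive an upward impulse, applied at world origin rather than the hit location.
; A hit does not destroy the bullet; only the lifetime timer does.
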(event EventBeginPlay
  (bind _self self)
  (Utilities|FlowControl|Delay 0.8)
  (Utilities|IsValid _self
    (:Is%20Valid
      (Actor|DestroyActor _self))))

(event Collision|EventHit
  (params (MyComp :type Primitive%20Component%20Object%20Reference) (Other :type Actor%20Object%20Reference) (OtherComp :type Primitive%20Component%20Object%20Reference) (bSelfMoved :type Boolean) (HitLocation :type Vector :default "0, 0, 0") (HitNormal :type Vector :default "0, 0, 0") (NormalImpulse :type Vector :default "0, 0, 0") (Hit :type Hit%20Result%20Structure%20%28by%20ref%29))
  (Audio|PlaySoundatLocation "/Game/Sounds/S_bullet_2.S_bullet_2" HitLocation "0, 0, 0" 1.0 1.0 0.0 0 0 0 0)
  (Utilities|FlowControl|Sequence
    (:then_0
      (Effects|SpawnEmitteratLocation "/Game/ExampleContent/Blueprint_Communication/Effects/P_Explosion_Bomb.P_Explosion_Bomb" HitLocation)
      (if (Utilities|DoesObjectImplementInterface Other "/Game/BluePrint/I_AirPlane.I_AirPlane_C")
        (Class|IAirPlane|Hit(Message) Other (Math|Conversions|ToFloat(Integer) (+ (Variables|Default|GetPowerHit) (Math|Random|RandomIntegerinRange 0 2))))))
    (:then_1
      (if (Physics|IsSimulatingPhysics OtherComp "None")
        (Physics|AddImpulseatLocation OtherComp "0.000000,0.000000,1333.000000" "0, 0, 0" "None")))))

(fn ConstructionScript)