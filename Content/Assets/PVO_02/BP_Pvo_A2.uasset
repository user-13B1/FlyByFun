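; Anti-aircraft gun turret that tracks and fires on the player's airplane once it comes within Eyesight distance.
; Each Tick while IsGame, it eases head yaw and trunk pitch toward the plane, using a Delay on Tick to pace fire.
; Firing spawns a dispersed BP_PVO2_Bullet at the Arrow while a timeline animates trunk recoil, head offset and ammo rotation.
; Hit passes power to the health widget; EndGame stops the turret.
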(event Custom|Fire
  ;[1 1 1] Comment
  (CallFunction|SpawnBullet)
  (bind _shot (Timeline|FireShot PlayFromStart)
    (:Update
      (Transformation|SetRelativeLocation (Variables|Default|GetSM_PvoGun_Trunk) (Math|Vector|Lerp(Vector) (Variables|Default|GetTrunkStartLocation) (Variables|Default|GetTrunkRecoilOffsetLocation) _shot) false false)
      (Transformation|SetRelativeRotation (Variables|Default|GetAmmoSet) (Math|Rotator|Lerp(Rotator) "0.000000,0.000000,-30.000000" "0, 0, 0" _shot) false false)
      (Transformation|SetRelativeLocation (Variables|Default|GetSM_PvoGun_Head) (Math|Vector|Lerp(Vector) "0.000000,0.000000,-10.000000" "0, 0, 0" _shot) false false))))

(event EventBeginPlay
  (bind _ascasual_air_plain_pawn (Utilities|Casting|CastToCasualAirPlainPawn (Game|Player|GetPlayerPawn 0)))
  (Variables|Default|SetAirPlainPawn _ascasual_air_plain_pawn))

(event Collision|EventActorBeginOverlap
  (params (OtherActor :type Actor%20Object%20Reference)))

(event EventTick
  (params (DeltaSeconds :type Float%20%28single-precision%29))
  (if (Variables|Default|GetIsGame)
    (bind _newparam (CallFunction|IsEyeSight))
    (if _newparam
      (CallFunction|UpdateHeadRotation DeltaSeconds)
      (CallFunction|UpdateArmsRotation DeltaSeconds)
      (Utilities|FlowControl|Delay (Variables|Default|GetDelayFire))
      (CallFunction|Fire)
      (Variables|Default|SetDelayFire (Variables|Default|GetRateFire)))))

(event EventEndGame
  (Variables|Default|SetIsGame false))

(event EventHit
  (params (Power :type Integer))
  (bind _asw_heals (Utilities|Casting|CastToW_Heals (UserInterface|GetWidget (Variables|Default|GetWidget))))
  (Default|SetHealsValue _asw_heals Power))

(fn ConstructionScript
  (bind _sm_pvogun_trunk (Variables|Default|GetSM_PvoGun_Trunk))
  (bind _relativelocation (Variables|/Script/Engine.SceneComponent|GetRelativeLocation _sm_pvogun_trunk))
  (bind (_x _y _z) (Math|Vector|BreakVector _relativelocation))
  (Variables|Default|SetTrunkStartLocation _relativelocation)
  (Variables|Default|SetTrunkRecoilOffsetLocation (Math|Vector|MakeVector (+ _x -4e+01) _y _z)))

(fn IsEyeSight
  (return (> (Variables|Default|GetEyesight) (Math|Vector|Distance(Vector) (Transformation|GetWorldLocation (Variables|Default|GetDefaultSceneRoot)) (Default|GetAirPlaneWorldLocation (Variables|Default|GetAirPlainPawn))))))

(fn UpdateHeadRotation
  (params (Delata :type Float%20%28double-precision%29))
  (Transformation|SetWorldRotation (Variables|Default|GetSM_PvoGun_Head) (Math|Rotator|MakeRotator 0.0 0.0 (.yaw (Math|Interpolation|RInterpTo (Transformation|GetWorldRotation (Variables|Default|GetSM_PvoGun_Head)) (Math|Rotator|FindLookatRotation (Transformation|GetWorldLocation (Variables|Default|GetSM_PvoGun_Head)) (Default|GetAirPlaneWorldLocation (Variables|Default|GetAirPlainPawn))) Delata 1.5))) false false))

(fn UpdateArmsRotation
  (params (Delta :type Float%20%28double-precision%29))
  (bind _sm_pvogun_trunk (Variables|Default|GetSM_PvoGun_Trunk))
  (Transformation|SetRelativeRotation (Variables|Default|GetSM_PvoGun_Trunk) (Math|Rotator|MakeRotator 0.0 (.pitch (Math|Interpolation|RInterpTo (Transformation|GetWorldRotation _sm_pvogun_trunk) (Math|Rotator|FindLookatRotation (Transformation|GetWorldLocation _sm_pvogun_trunk) (Transformation|GetActorLocation (Game|Player|GetPlayerPawn 0))) Delta 2.0)) 0.0) false false))

(fn SpawnBullet
  (bind _arrow (Variables|Default|GetArrow))
  (bind _outpurroll (CallFunction|AddBulletDispersion 0.3 (Transformation|GetWorldRotation _arrow)))
  (Game|SpawnActorfromClass "/Game/Assets/PVO_02/BP_PVO2_Bullet.BP_PVO2_Bullet_C" (Math|Transform|MakeTransform (Transformation|GetWorldLocation _arrow) _outpurroll) "AdjustIfPossibleButDontSpawnIfColliding" 0 0))