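; BP_Gate is a single-use pickup gate with Blue and Red trigger components that grant effects to airplanes.
; The first overlap on either trigger clears IsActive, without checking which actor entered.
; Blue sends AddGunAmmo and Red sends Treat, both broadcast to every I_AirPlane actor in the world rather than just the overlapping one.
; Both branches share a step inside their loops that hides the SMGates mesh.
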(event OnComponentBeginOverlap(Blue)
  (params (OverlappedComponent :type Primitive%20Component%20Object%20Reference) (OtherActor :type Actor%20Object%20Reference) (OtherComp :type Primitive%20Component%20Object%20Reference) (OtherBodyIndex :type Integer) (bFromSweep :type Boolean) (SweepResult :type Hit%20Result%20Structure%20%28by%20ref%29))
  (if (Variables|Default|GetIsActive)
    (Variables|Default|SetIsActive false)
    (bind _outactors (Actor|GetAllActorswithInterface "/Game/AirPlane/I_AirPlane.I_AirPlane_C"))
    (for _array_element _outactors
      (Class|IAirPlane|AddGunAmmo(Message) _array_element 120)
      (Rendering|SetVisibility (Variables|Default|GetSM_Gates) false false))))

(event OnComponentBeginOverlap(Red)
  (params (OverlappedComponent :type Primitive%20Component%20Object%20Reference) (OtherActor :type Actor%20Object%20Reference) (OtherComp :type Primitive%20Component%20Object%20Reference) (OtherBodyIndex :type Integer) (bFromSweep :type Boolean) (SweepResult :type Hit%20Result%20Structure%20%28by%20ref%29))
  (if (Variables|Default|GetIsActive)
    (Variables|Default|SetIsActive false)
    (bind _outactors (Actor|GetAllActorswithInterface "/Game/AirPlane/I_AirPlane.I_AirPlane_C"))
    (for _array_element _outactors
      (Class|IAirPlane|Treat(Message) _array_element 0.0 40)
      (Rendering|SetVisibility (Variables|Default|GetSM_Gates) false false))))

(fn ConstructionScript)